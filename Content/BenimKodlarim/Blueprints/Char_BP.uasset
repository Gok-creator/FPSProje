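; Player character with yaw-relative movement and controls to open, peek through and interact with doors.
; BeginPlay caches one LockDoor_BP and one OpenDoor_BP, and the open and peek keys trigger both through Replicate-named events.
; Holding E while IsInside runs a timeline that, on completion, calls Epress on the still-locked door.
; Capsule overlaps with tagged actors manage door widgets for the locally controlled player only.
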(event `self.ReceiveBeginPlay`
  (bind _returnvalue (`GameplayStatics.GetActorOfClass` "/Game/BenimKodlarim/Blueprints/Object/LockDoor_BP.LockDoor_BP_C"))
  (set `self.DoorRef` _returnvalue)
  (bind _returnvalue_2 (`GameplayStatics.GetActorOfClass` "/Game/BenimKodlarim/Blueprints/Object/OpenDoor_BP.OpenDoor_BP_C"))
  (set `self.openDoorRef` _returnvalue_2))

(event `InputAxis|InputForward`
  (params (AxisValue :type "Float (single-precision)"))
  ;[1 1 1] Movement
  (`self.AddMovementInput` (`KismetMathLibrary.GetForwardVector` (`KismetMathLibrary.MakeRotator` 0.0 0.0 (.yaw (`Controller.GetControlRotation` (`GameplayStatics.GetPlayerController` 0))))) AxisValue))

(event `InputAxis|InputRight`
  (params (AxisValue :type "Float (single-precision)"))
  ;[1 1 1] Movement
  (`self.AddMovementInput` (`KismetMathLibrary.GetRightVector` (`KismetMathLibrary.MakeRotator` 0.0 0.0 (.yaw (`Controller.GetControlRotation` (`GameplayStatics.GetPlayerController` 0))))) AxisValue))

(event `InputAxis|LookRight`
  (params (AxisValue :type "Float (single-precision)"))
  ;[1 1 1] mouse
  (`self.AddControllerYawInput` AxisValue))

(event `InputAction|PeakDoorKey`
  (params (Key :type "Key Structure"))
  ;[1 1 1] Dispatcher
  (:`Pressed`
    (`self.ReplicateFunctionTInput`)))

(event `ReplicateFunctionFInput`
  (bind _opendoorref (`self.openDoorRef`))
  (bind _doorref (`self.DoorRef`))
  ;[1 1 1] Replication
  (`/Engine/EditorBlueprintResources/StandardMacros.IsValid` _opendoorref
    (:`Is Valid`
      (`/Game/BenimKodlarim/Blueprints/Object/OpenDoor_BP.ReplicationOpenDoor` _opendoorref)
      (`/Engine/EditorBlueprintResources/StandardMacros.IsValid` _doorref
        (:`Is Valid`
          (`/Game/BenimKodlarim/Blueprints/Object/LockDoor_BP.ReplicationLockOpenDoor` _doorref)
          (`KismetSystemLibrary.PrintString` (`KismetSystemLibrary.GetDisplayName` self)))))))

(event `InputAction|OpenDoorKey`
  (params (Key :type "Key Structure"))
  ;[1 1 1] Dispatcher
  (:`Pressed`
    (`self.ReplicateFunctionFInput`)))

(event `ReplicateFunctionTInput`
  (bind _opendoorref (`self.openDoorRef`))
  (bind _doorref (`self.DoorRef`))
  ;[1 1 1] Replication
  (`/Engine/EditorBlueprintResources/StandardMacros.IsValid` _opendoorref
    (:`Is Valid`
      (`/Game/BenimKodlarim/Blueprints/Object/OpenDoor_BP.ReplicationPeakDoor` _opendoorref)
      (`/Engine/EditorBlueprintResources/StandardMacros.IsValid` _doorref
        (:`Is Valid`
          (`/Game/BenimKodlarim/Blueprints/Object/LockDoor_BP.ReplicationLockPeakDoor` _doorref)
          (`KismetSystemLibrary.PrintString` (`KismetSystemLibrary.GetDisplayName` self)))))))

(event `InputAction|pressE`
  (params (Key :type "Key Structure"))
  (bind _isinside (`self.isInside`))
  ;[1 1 1] Dispatcher
  (:`Pressed`
    (if _isinside
      (if (not (`/Game/BenimKodlarim/Blueprints/Object/LockDoor_BP.unlocked` (`self.DoorRef`)))
        (set `self.ePress` true)
        (bind (_direction _ispress) (`Timeline|PressETimeLine` :!label _label)
          (:`Finished`
            (if (== _ispress 1.0)
              (`self.ReplicateFunctionEInput`)))))))
  (:`Released`
    (if _isinside
      (set `self.ePress` false)
      (goto _label :!via `Stop`))))

(event `ReplicateFunctionEInput`
  ;[1 1 1] Replication
  (`/Game/BenimKodlarim/Blueprints/Object/LockDoor_BP.Epress` (`self.DoorRef`)))

(event `DoorWidgetOpen`
  ;[1 1 1] DoorWidget
  ;;[0 0.05694 1] Open Door
  (if (`self.IsLocallyControlled`)
    (bind _returnvalue (`|CreateWidget` "/Game/BenimKodlarim/Blueprints/Widget/kapiUI_WG.kapiUI_WG_C" (`GameplayStatics.GetPlayerController` 0)))
    (`UserWidget.AddToPlayerScreen` _returnvalue 0)))

(event `self.CapsuleComponent.OnComponentBeginOverlap`
  (params (OverlappedComponent :type "PrimitiveComponent Object Reference") (OtherActor :type "Actor Object Reference") (OtherComp :type "PrimitiveComponent Object Reference") (OtherBodyIndex :type Integer) (bFromSweep :type Boolean) (SweepResult :type "HitResult Structure (by ref)"))
  ;[1 1 1] Collisionlar
  (`|ExecutionSequence`
    (:`then_0`
      (if (`self.ActorHasTag` OtherActor "OpenDoor")
        (`self.DoorWidgetOpen`)))
    (:`then_1`
      (if (`self.ActorHasTag` OtherActor "LockDoor")
        (if (`/Game/BenimKodlarim/Blueprints/Object/LockDoor_BP.unlocked` (`self.DoorRef`))
          _
          (elif (`/Game/BenimKodlarim/Blueprints/Object/LockDoor_BP.isLock` (`self.DoorRef`))
            (`self.DoorLocked`)))))))

(event `DoorWidgetClose`
  ;[1 1 1] DoorWidget
  ;;[0 0.05694 1] Open Door
  (`/Engine/EditorBlueprintResources/StandardMacros.IsValid` (stale `DoorWidgetOpen` _returnvalue)
    (:`Is Valid`
      (`Widget.RemoveFromParent` (stale `DoorWidgetOpen` _returnvalue)))))

(event `DoorLocked`
  ;[1 1 1] DoorWidget
  ;;[1 0.1288 0] LockDoor
  (if (`self.IsLocallyControlled`)
    (`/Game/BenimKodlarim/Blueprints/Object/LockDoor_BP.LockDoorWidgetEvent` (`self.DoorRef`))))

(event `self.CapsuleComponent.OnComponentEndOverlap`
  (params (OverlappedComponent :type "PrimitiveComponent Object Reference") (OtherActor :type "Actor Object Reference") (OtherComp :type "PrimitiveComponent Object Reference") (OtherBodyIndex :type Integer))
  ;[1 1 1] Collisionlar
  (`|ExecutionSequence`
    (:`then_0`
      (if (`self.ActorHasTag` OtherActor "OpenDoor")
        (`self.DoorWidgetClose`)))
    (:`then_1`
      (if (`self.ActorHasTag` OtherActor "LockDoor")
        (if (`/Game/BenimKodlarim/Blueprints/Object/LockDoor_BP.unlocked` (`self.DoorRef`))
          (`self.DoorUnlocked`))))))

(event `DoorUnlocked`
  ;[1 1 1] DoorWidget
  ;;[1 0.1288 0] LockDoor
  (if (`self.IsLocallyControlled`)
    _))

(fn `UserConstructionScript`)