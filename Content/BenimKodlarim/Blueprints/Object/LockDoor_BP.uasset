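; Lockable door actor that the player can peek through or swing open once an E-press event unlocks it.
; A trigger box sets open and peek flags on the Char_BP found at BeginPlay and clears prompt widgets on exit.
; Replication-named events feed the open and peek handlers, whose timelines rotate the door's yaw based on shared state and current angle.
; Unlocking swaps the lock prompt for the door prompt; direct character input bindings are disconnected.
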(event `ReplicationLockPeakDoor`
  ;[1 1 1] Begin Play
  (`self.BindDispatcher2`))

(event `ReplicationLockOpenDoor`
  ;[1 1 1] Begin Play
  (`self.BindDispatcher`))

(event `self.ReceiveBeginPlay`
  (bind _charref_0 (`self.charRef_0`))
  ;[1 1 1] Begin Play
  (bind _returnvalue (`GameplayStatics.GetActorOfClass` "/Game/BenimKodlarim/Blueprints/Char_BP.Char_BP_C"))
  (set `self.charRef_0` _returnvalue)
  (`/Game/BenimKodlarim/Blueprints/Char_BP.ReplicateFunctionFInput` _charref_0)
  (`/Game/BenimKodlarim/Blueprints/Char_BP.ReplicateFunctionTInput` _charref_0))

(event `BindDispatcher`
  ;[1 1 1] Replicate
  (`self.OpenDispatcher`))

(event `PeakDispatcher`
  (bind _cube (`self.Cube`))
  ;[1 1 1] Peak Dispatcher
  (if (`self.unlocked`)
    (if (`|GetArrayItem` (`/Game/BenimKodlarim/Blueprints/Char_BP.isPeak` (`self.charRef_0`)) 1)
      (if (== (`self.oTimeLineSorgu`) true)
        (`/Engine/EditorBlueprintResources/StandardMacros.FlipFlop`
          (:`A`
            (bind (_direction _peakdoor) (`Timeline|PeakTimeLine` :!via `PlayFromStart` :!label _label)
              (:`Update`
                (`SceneComponent.K2_SetRelativeRotation` _cube (`KismetMathLibrary.MakeRotator` 0.0 0.0 _peakdoor) false false)
                (if (== _peakdoor 30.0)
                  (set `self.pTimeLineSorgu` true)
                  (else
                    (set `self.pTimeLineSorgu` false))))))
          (:`B`
            (goto _label :!via `ReverseFromEnd`)))
        (else
          (bind (_direction_2 _peakdoor_2) (`Timeline|Timeline_1` :!via `PlayFromStart`)
            (:`Update`
              (`SceneComponent.K2_SetRelativeRotation` _cube (`KismetMathLibrary.MakeRotator` 0.0 0.0 _peakdoor_2) false false)
              (set `self.oTimeLineSorgu` true))))))))

(event `BindDispatcher2`
  ;[1 1 1] Replicate
  (`self.PeakDispatcher`))

(event `OpenDispatcher`
  (bind _cube (`self.Cube`))
  (bind (_relativerotation_roll _relativerotation_pitch _relativerotation_yaw) (`KismetMathLibrary.BreakRotator` (`SceneComponent.RelativeRotation` _cube)))
  ;[1 1 1] Open Dispatcher
  (set `self.actorRotation` _relativerotation_yaw)
  (if (`self.unlocked`)
    (if (`|GetArrayItem` (`/Game/BenimKodlarim/Blueprints/Char_BP.isOpen` (`self.charRef_0`)) 1)
      (if (`self.oTimeLineSorgu`)
        (set `self.oTimeLineSorgu` false)
        (bind (_direction _opendoor) (`Timeline|OpenTimeLine` :!via `PlayFromStart` :!label _label_2)
          (:`Update`
            (`SceneComponent.K2_SetRelativeRotation` _cube (`KismetMathLibrary.MakeRotator` 0.0 0.0 _opendoor) false false))
          (:`Finished`
            (if (== _opendoor 120.0)
              (set `self.oTimeLineSorgu` false)
              (else
                (set `self.oTimeLineSorgu` true)))))
        (elif (== (stale `PeakDispatcher` _peakdoor_2) 15.0)
          (bind (_direction_2 _peakdoor) (`Timeline|Timeline_0` :!via `PlayFromStart`)
            (:`Update`
              (`SceneComponent.K2_SetRelativeRotation` _cube (`KismetMathLibrary.MakeRotator` 0.0 0.0 _peakdoor) false false)
              (set `self.oTimeLineSorgu` false)))
          (elif (== _opendoor 120.0)
            (goto _label_2 :!via `ReverseFromEnd`)))))))

(event `Epress`
  ;[1 1 1] E press Dispatcher
  (set `self.unlocked` true)
  (`self.UnlockEvent`))

(event `UnlockEvent`
  ;[1 1 1] Unlock
  (`/Engine/EditorBlueprintResources/StandardMacros.IsValid` (stale `LockDoorWidgetEvent` _returnvalue)
    (:`Is Valid`
      (`Widget.RemoveFromParent` (stale `LockDoorWidgetEvent` _returnvalue))
      (bind _returnvalue (`|CreateWidget` "/Game/BenimKodlarim/Blueprints/Widget/kapiUI_WG.kapiUI_WG_C"))
      (`UserWidget.AddToViewport` _returnvalue 0))))

(event `self.Box.OnComponentBeginOverlap`
  (params (OverlappedComponent :type "PrimitiveComponent Object Reference") (OtherActor :type "Actor Object Reference") (OtherComp :type "PrimitiveComponent Object Reference") (OtherBodyIndex :type Integer) (bFromSweep :type Boolean) (SweepResult :type "HitResult Structure (by ref)"))
  (bind _charref_0 (`self.charRef_0`))
  ;[1 1 1] Begin Overlap
  (if (`self.ActorHasTag` OtherActor "Player")
    (`KismetArrayLibrary.Array_Set` (`/Game/BenimKodlarim/Blueprints/Char_BP.isOpen` _charref_0) 1 true)
    (`KismetArrayLibrary.Array_Set` (`/Game/BenimKodlarim/Blueprints/Char_BP.isPeak` _charref_0) 1 true)
    (set `/Game/BenimKodlarim/Blueprints/Char_BP.isInside` true _charref_0)
    (if (`self.unlocked`)
      _)))

(event `WidgetEvent`
  ;[1 1 1] Events UI
  (bind _returnvalue (`|CreateWidget` "/Game/BenimKodlarim/Blueprints/Widget/kapiUI_WG.kapiUI_WG_C"))
  (`UserWidget.AddToPlayerScreen` _returnvalue 0))

(event `LockDoorWidgetEvent`
  ;[1 1 1] Events UI
  (if (`Pawn.IsLocallyControlled` (`GameplayStatics.GetPlayerCharacter` 0))
    (bind _returnvalue (`|CreateWidget` "/Game/BenimKodlarim/Blueprints/Widget/LockDoorUI_WG.LockDoorUI_WG_C"))
    (`UserWidget.AddToPlayerScreen` _returnvalue 0)))

(event `self.Box.OnComponentEndOverlap`
  (params (OverlappedComponent :type "PrimitiveComponent Object Reference") (OtherActor :type "Actor Object Reference") (OtherComp :type "PrimitiveComponent Object Reference") (OtherBodyIndex :type Integer))
  (bind _charref_0 (`self.charRef_0`))
  ;[1 1 1] End Overlap
  (if (`self.ActorHasTag` OtherActor "Player")
    (`KismetArrayLibrary.Array_Set` (`/Game/BenimKodlarim/Blueprints/Char_BP.isOpen` _charref_0) 1)
    (`KismetArrayLibrary.Array_Set` (`/Game/BenimKodlarim/Blueprints/Char_BP.isPeak` _charref_0) 1)
    (`/Engine/EditorBlueprintResources/StandardMacros.IsValid` _charref_0
      (:`Is Valid`
        (set `/Game/BenimKodlarim/Blueprints/Char_BP.isInside` false _charref_0)
        (if (`self.unlocked`)
          (`|ExecutionSequence`
            (:`then_0`
              (`/Engine/EditorBlueprintResources/StandardMacros.IsValid` (stale `UnlockEvent` _returnvalue)
                (:`Is Valid`
                  (`Widget.RemoveFromParent` (stale `UnlockEvent` _returnvalue)))))
            (:`then_1`
              (`/Engine/EditorBlueprintResources/StandardMacros.IsValid` (stale `WidgetEvent` _returnvalue)
                (:`Is Valid`
                  (`Widget.RemoveFromParent` (stale `WidgetEvent` _returnvalue))))))
          (else
            (`|ExecutionSequence`
              (:`then_0`
                (`/Engine/EditorBlueprintResources/StandardMacros.IsValid` (stale `LockDoorWidgetEvent` _returnvalue)
                  (:`Is Valid`
                    (`Widget.RemoveFromParent` (stale `LockDoorWidgetEvent` _returnvalue)))))
              (:`then_1`
                (`/Engine/EditorBlueprintResources/StandardMacros.IsValid` (stale `WidgetEvent` _returnvalue)
                  (:`Is Valid`
                    (`Widget.RemoveFromParent` (stale `WidgetEvent` _returnvalue))))))))))))

(fn `OpenInput`)

(fn `PeakInput`)

(fn `UserConstructionScript`)