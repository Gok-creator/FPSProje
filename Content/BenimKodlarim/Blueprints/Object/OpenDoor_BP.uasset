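; Door actor that the player can peek through or swing open, animated by timelines that set the Cube's yaw.
; A trigger box sets the IsPeak and IsOpen flags on a Char_BP found at BeginPlay as Player-tagged actors enter or leave.
; Authority-gated events run the peek and open logic, which checks those flags and door state to pick a timeline.
; The direct input-binding calls to the character are disconnected.
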(event `ReplicationPeakDoor`
  ;[1 1 1] Begin Play
  (`/Engine/EditorBlueprintResources/ActorMacros.Switch Has Authority`
    (:`Authority`
      (`self.BindDispatcher2`))))

(event `ReplicationOpenDoor`
  ;[1 1 1] Begin Play
  (`/Engine/EditorBlueprintResources/ActorMacros.Switch Has Authority`
    (:`Authority`
      (`self.BindDispatcher`))))

(event `self.ReceiveBeginPlay`
  (bind _cref (`self.cRef`))
  ;[1 1 1] Begin Play
  (bind _returnvalue (`GameplayStatics.GetActorOfClass` "/Game/BenimKodlarim/Blueprints/Char_BP.Char_BP_C"))
  (set `self.cRef` _returnvalue)
  (`/Game/BenimKodlarim/Blueprints/Char_BP.ReplicateFunctionFInput` _cref)
  (`/Game/BenimKodlarim/Blueprints/Char_BP.ReplicateFunctionTInput` _cref))

(event `BindDispatcher`
  ;[1 1 1] Replication
  (`self.OpenInput`))

(event `PeakInput`
  (bind _cube (`self.Cube`))
  ;[1 1 1] Peak Dispatcher
  (if (`|GetArrayItem` (`/Game/BenimKodlarim/Blueprints/Char_BP.isPeak` (`self.cRef`)))
    (if (== (`self.oTimelineSorgu`) true)
      (`/Engine/EditorBlueprintResources/StandardMacros.FlipFlop`
        (:`A`
          (bind (_direction _peakdoor) (`Timeline|Timeline_2` :!via `PlayFromStart` :!label _label)
            (:`Update`
              (`SceneComponent.K2_SetRelativeRotation` _cube (`KismetMathLibrary.MakeRotator` 0.0 0.0 _peakdoor) false false)
              (if (== _peakdoor 30.0)
                (set `self.pTimeLineSorgu` true)
                (else
                  (set `self.pTimeLineSorgu` false))))))
        (:`B`
          (goto _label :!via `ReverseFromEnd`)))
      (else
        (bind (_direction_2 _peakdoor_2) (`Timeline|Timeline_4` :!via `PlayFromStart`)
          (:`Update`
            (`SceneComponent.K2_SetRelativeRotation` _cube (`KismetMathLibrary.MakeRotator` 0.0 0.0 _peakdoor_2) false false)
            (set `self.oTimelineSorgu` true)))))))

(event `BindDispatcher2`
  ;[1 1 1] Replication
  (`self.PeakInput`))

(event `OpenInput`
  (bind _cube (`self.Cube`))
  (bind _cref (`self.cRef`))
  ;[1 1 1] Open Dispatcher
  (`/Engine/EditorBlueprintResources/StandardMacros.IsValid` _cref
    (:`Is Valid`
      (if (`|GetArrayItem` (`/Game/BenimKodlarim/Blueprints/Char_BP.isOpen` _cref))
        (if (`self.oTimelineSorgu`)
          (set `self.oTimelineSorgu` false)
          (bind (_direction _opendoor) (`Timeline|Timeline_3` :!via `PlayFromStart` :!label _label_2)
            (:`Update`
              (`SceneComponent.K2_SetRelativeRotation` _cube (`KismetMathLibrary.MakeRotator` 0.0 0.0 _opendoor) false false))
            (:`Finished`
              (if (== _opendoor 120.0)
                (set `self.oTimelineSorgu` false)
                (else
                  (set `self.oTimelineSorgu` true)))))
          (elif (== (stale `PeakInput` _peakdoor_2) 15.0)
            (bind (_direction_2 _peakdoor) (`Timeline|Timeline_5` :!via `PlayFromStart`)
              (:`Update`
                (`SceneComponent.K2_SetRelativeRotation` _cube (`KismetMathLibrary.MakeRotator` 0.0 0.0 _peakdoor) false false)
                (set `self.oTimelineSorgu` false)))
            (elif (== _opendoor 120.0)
              (goto _label_2 :!via `ReverseFromEnd`))))))))

(event `self.Box.OnComponentBeginOverlap`
  (params (OverlappedComponent :type "PrimitiveComponent Object Reference") (OtherActor :type "Actor Object Reference") (OtherComp :type "PrimitiveComponent Object Reference") (OtherBodyIndex :type Integer) (bFromSweep :type Boolean) (SweepResult :type "HitResult Structure (by ref)"))
  ;[1 1 1] Lapı Collision işlemleri
  (if (`self.ActorHasTag` OtherActor "Player")
    (`self.CollisionBegin`)))

(event `self.Box.OnComponentEndOverlap`
  (params (OverlappedComponent :type "PrimitiveComponent Object Reference") (OtherActor :type "Actor Object Reference") (OtherComp :type "PrimitiveComponent Object Reference") (OtherBodyIndex :type Integer))
  ;[1 1 1] Lapı Collision işlemleri
  (if (`self.ActorHasTag` OtherActor "Player")
    (`self.CollisionEnd`)))

(event `CollisionBegin`
  (bind _cref (`self.cRef`))
  ;[1 1 1] Collision Custom Event
  (`/Engine/EditorBlueprintResources/StandardMacros.IsValid` _cref
    (:`Is Valid`
      (`KismetArrayLibrary.Array_Set` (`/Game/BenimKodlarim/Blueprints/Char_BP.isPeak` _cref) 0 true)
      (`KismetArrayLibrary.Array_Set` (`/Game/BenimKodlarim/Blueprints/Char_BP.isOpen` _cref) 0 true))))

(event `CollisionEnd`
  (bind _cref (`self.cRef`))
  ;[1 1 1] Collision Custom Event
  (`/Engine/EditorBlueprintResources/StandardMacros.IsValid` _cref
    (:`Is Valid`
      (`KismetArrayLibrary.Array_Set` (`/Game/BenimKodlarim/Blueprints/Char_BP.isPeak` _cref))
      (`KismetArrayLibrary.Array_Set` (`/Game/BenimKodlarim/Blueprints/Char_BP.isOpen` _cref)))))

(fn `UserConstructionScript`)